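; Anim notify that conditionally advances the player's montage to a configured NextSection, apparently to chain combat combo animations.
; When fired, it casts the mesh owner to BP_PlayerPawn and asks its CombatComponent whether it can switch to that section.
; If allowed, the mesh's anim instance jumps to the section.
; Disconnected nodes hold an unused ABP_Xbot combo-update path with frame counting and a None-section check.
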(fn `Received_Notify`
  (params (MeshComp :type "SkeletalMeshComponent Object Reference") (Animation :type "AnimSequenceBase Object Reference"))
  (returns (ReturnValue :type Boolean))
  (bind _nextsection (`self.NextSection`))
  (bind _asbp_player_pawn (cast `/Game/Blueprints/BP_PlayerPawn` (`ActorComponent.GetOwner` MeshComp)))
  (bind _canswitch (`/Game/Blueprints/BP_CombatComponent.CanSwitchToMontageSection` (`/Game/Blueprints/BP_PlayerPawn.CombatComponent` _asbp_player_pawn) _nextsection))
  (if _canswitch
    (`AnimInstance.Montage_JumpToSection` (`SkeletalMeshComponent.GetAnimInstance` MeshComp) _nextsection null)))