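; BP_HurricaneKickAttack is a player attack that repeats a looping kick while its button is held, then ends with a finisher.
; Each animation section update counts a loop and refreshes the combat component's attack direction.
; On button release or at the loop limit, it switches the montage to its End section and sets Finish.
; The finisher overrides the parent's forces with fixed pushback and boosted knockup.
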(fn `GetPushbackAndKnockupForces`
  (returns (PushbackForce :type "Float (double-precision)") (KnockupForce :type "Float (double-precision)"))
  (bind (_pushbackforce _knockupforce) (`parent.GetPushbackAndKnockupForces`))
  (if (`self.Finish`)
    (return 800.0 (* (`AttackData.KnockupForce` (`self.AttackData`)) 1.5)) ; Finisher attack
    (else
      (return _pushbackforce _knockupforce))))

(fn `UpdateAnimSectionStatus`
  (bind _playerpawn (`self.PlayerPawn`))
  (`|ExecutionSequence`
    (:`then_0`
      (`/Engine/EditorBlueprintResources/StandardMacros.IncrementInt` (`self.NumLoops`)
        (:`  `
          (`/Game/Blueprints/BP_CombatComponent.UpdateAttackDirection` (`/Game/Blueprints/BP_PlayerPawn.CombatComponent` _playerpawn)))))
    (:`then_1`
      (if (or (>= (`self.NumLoops`) (`self.MaxNumLoops`)) (not (`/Game/Blueprints/BP_PlayerPawnController.IsButtonHeld` (`/Game/Blueprints/BP_PlayerPawn.PlayerPawnController` _playerpawn) "NewEnumerator2")))
        (set `self.CurrentMontageSection` "End")
        (set `self.Finish` true)))))

(fn `UserConstructionScript`)