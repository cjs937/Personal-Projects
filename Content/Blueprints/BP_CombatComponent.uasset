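; Player combat component that runs attacks as spawned attack actors, one at a time.
; BeginAttack requests the attack state, turns the mesh toward movement input (or keeps its facing), replaces the current attack with one attached to the mesh, and plays its montage from the attack data.
; An uninterrupted montage end returns the player to idle, resets the combo and destroys the attack.
; Helper functions query and update the current attack's montage section.
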(event `self.ReceiveBeginPlay`
  (bind _asbp_player_pawn (cast `/Game/Blueprints/BP_PlayerPawn` (`GameplayStatics.GetPlayerPawn` 0)))
  (bind _output_get (set `self.OwnerPlayerPawn` _asbp_player_pawn))
  (add `AnimInstance.OnMontageEnded` (`SkeletalMeshComponent.GetAnimInstance` (`PlayerPawn.SkeletalMesh` _output_get)) (delegate `OnMontageCompleted`)))

(event `OnMontageCompleted`
  (params (Montage :type "AnimMontage Object Reference") (bInterrupted :type Boolean))
  (bind _currentattack (`self.CurrentAttack`))
  (if (not bInterrupted)
    (`StateMachine.Request` (`PlayerPawn.PlayerStateMachine` (`self.OwnerPlayerPawn`)) "/Script/PilgrimageUnreal.PlayerIdleState")
    (`/Game/Blueprints/BP_PlayerPawn.ResetCombo` (`self.OwnerPlayerPawn`))
    (`/Engine/EditorBlueprintResources/StandardMacros.IsValid` _currentattack
      (:`Is Valid`
        (`Actor.K2_DestroyActor` _currentattack)))))

(fn `BeginAttack`
  (params (AttackClass :type "/Game/Blueprints/BP_Attack Class Reference") (AttackData :type "AttackData Object Reference"))
  (bind _spawnoffset (`AttackData.SpawnOffset` AttackData))
  (bind _ownerplayerpawn (`self.OwnerPlayerPawn`))
  (bind _currentattack (`self.CurrentAttack`))
  (bind _attachtosocketname (`AttackData.AttachToSocketName` AttackData))
  (bind _playerstatemachine (`PlayerPawn.PlayerStateMachine` (`self.OwnerPlayerPawn`)))
  (bind _returnvalue (`SkeletalMeshComponent.GetAnimInstance` (`PlayerPawn.SkeletalMesh` (`self.OwnerPlayerPawn`))))
  (bind (_returnvalue_location _returnvalue_rotation _returnvalue_scale) (`KismetMathLibrary.BreakTransform` (`SceneComponent.K2_GetComponentToWorld` (`/Game/Blueprints/BP_PlayerPawn.DefaultHitboxLocation` (`self.OwnerPlayerPawn`)))))
  (bind (_returnvalue_location_2 _returnvalue_rotation_2 _returnvalue_scale_2) (`KismetMathLibrary.BreakTransform` (`SceneComponent.GetSocketTransform` (`PlayerPawn.SkeletalMesh` _ownerplayerpawn) _attachtosocketname "RTS_World")))
  (bind _returnvalue_location_3 (`KismetMathLibrary.BreakTransform` (select `bool` (== _attachtosocketname "None") :`false` (`KismetMathLibrary.MakeTransform` (+ _returnvalue_location_2 _spawnoffset) _returnvalue_rotation_2 _returnvalue_scale_2) :`true` (`KismetMathLibrary.MakeTransform` (+ _returnvalue_location _spawnoffset) _returnvalue_rotation _returnvalue_scale))))
  (`|ExecutionSequence`
    (:`then_0`
      (cast `/Game/Blueprints/BP_PlayerAttackState` (`StateMachine.GetCurrentState` _playerstatemachine)
        (:`CastFailed`
          (`StateMachine.Request` _playerstatemachine "/Game/Blueprints/BP_PlayerAttackState.BP_PlayerAttackState_C"))))
    (:`then_1`
      (`self.UpdateAttackDirection`)
      (`/Engine/EditorBlueprintResources/StandardMacros.IsValid` _currentattack
        (:`Is Valid`
          (`Actor.K2_DestroyActor` _currentattack))))
    (:`then_2`
      (set `/Game/Blueprints/BP_PlayerPawn.CanCancel` false _ownerplayerpawn)
      (if (and (`KismetSystemLibrary.IsValidClass` AttackClass) (`KismetSystemLibrary.IsValid` AttackData))
        (bind _returnvalue_2 (`|SpawnActorFromClass` AttackClass (`KismetMathLibrary.MakeTransform` _returnvalue_location_3 (struct) (`AttackData.ScaleOverride` AttackData)) "Undefined" "OverrideRootScale" null (`self.OwnerPlayerPawn`) AttackData (`self.AttackDirection`) null))
        (`SceneComponent.SetAbsolute` (`/Game/Blueprints/BP_Attack.DefaultSceneRoot` _returnvalue_2) false true true)
        (bind _output_get (set `self.CurrentAttack` _returnvalue_2))
        (bind _attackdata (`/Game/Blueprints/BP_Attack.AttackData` _returnvalue_2))
        (`Actor.K2_AttachToComponent` _output_get (`PlayerPawn.SkeletalMesh` (`self.OwnerPlayerPawn`)) (`AttackData.AttachToSocketName` _attackdata) "KeepWorld" "KeepRelative" "KeepWorld" true)
        (`/Engine/EditorBlueprintResources/StandardMacros.IsValid` (`AttackData.Animation` _attackdata)
          (:`Is Valid`
            (`AnimInstance.Montage_Stop` _returnvalue 0.0 null)
            (`AnimInstance.Montage_Play` _returnvalue (`AttackData.Animation` (`local.AttackData`)) 1.0 "MontageLength" 0.0 true)))))))

(fn `CanSwitchToMontageSection`
  (params (NextSection :type Name))
  (returns (CanSwitch :type Boolean))
  (bind _currentattack (`self.CurrentAttack`))
  (`/Engine/EditorBlueprintResources/StandardMacros.IsValid` _currentattack
    (:`Is Valid`
      (return (== NextSection (`/Game/Blueprints/BP_Attack.CurrentMontageSection` _currentattack))))))

(fn `Reset`
  (bind _currentattack (`self.CurrentAttack`))
  (set `self.CurrentComboCount` 0)
  (`/Engine/EditorBlueprintResources/StandardMacros.IsValid` _currentattack
    (:`Is Valid`
      (`Actor.K2_DestroyActor` _currentattack))))

(fn `UpdateAttackDirection`
  (bind _currentattack (`self.CurrentAttack`))
  (bind _ownerplayerpawn (`self.OwnerPlayerPawn`))
  (bind _skeletalmesh (`PlayerPawn.SkeletalMesh` _ownerplayerpawn))
  (bind (_returnvalue_roll _returnvalue_pitch) (`KismetMathLibrary.BreakRotator` (`SceneComponent.K2_GetComponentRotation` _skeletalmesh)))
  (bind _returnvalue (`PlayerPawn.GetMoveDirection` _ownerplayerpawn))
  (bind _output_get (set `self.AttackDirection` (`KismetMathLibrary.SelectVector` (`SceneComponent.GetForwardVector` _skeletalmesh) _returnvalue (== _returnvalue (`KismetMathLibrary.Vector_Zero`)))))
  (bind (_returnvalue_roll_2 _returnvalue_pitch_2 _returnvalue_yaw) (`KismetMathLibrary.BreakRotator` (`KismetMathLibrary.FindLookAtRotation` (`KismetMathLibrary.Vector_Zero`) _output_get)))
  (`SceneComponent.K2_SetWorldRotation` _skeletalmesh (`KismetMathLibrary.MakeRotator` _returnvalue_roll _returnvalue_pitch _returnvalue_yaw) false false)
  (`/Engine/EditorBlueprintResources/StandardMacros.IsValid` _currentattack
    (:`Is Valid`
      (set `/Game/Blueprints/BP_Attack.Direction` (`self.AttackDirection`) _currentattack))))

(fn `UpdateMontageSectionStatus`
  (bind _currentattack (`self.CurrentAttack`))
  (`/Engine/EditorBlueprintResources/StandardMacros.IsValid` _currentattack
    (:`Is Valid`
      (`/Game/Blueprints/BP_Attack.UpdateAnimSectionStatus` _currentattack)
      (return))))