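; Player state machine state that holds the pawn in the Attacking locomotion state.
; Entering disables movement; exiting restores it, stops montages instantly, re-enables cancelling, and resets the combo and CombatComponent.
; BeginAttack is empty; the logic for aiming, spawning attack actors, playing montages and returning to idle is disconnected and never runs.
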(event `self.EnterState`
  (bind _playerpawn (`self.PlayerPawn`))
  (`PlayerPawn.SetMovementAllowed` _playerpawn false)
  (`PlayerPawn.SetLocomotionState` _playerpawn "Attacking"))

(event `self.ExitState`
  (bind _playerpawn (`self.PlayerPawn`))
  (`PlayerPawn.SetMovementAllowed` _playerpawn true)
  (`AnimInstance.Montage_Stop` (`SkeletalMeshComponent.GetAnimInstance` (`PlayerPawn.SkeletalMesh` _playerpawn)) 0.0 null)
  (bind _asbp_player_pawn (cast `/Game/Blueprints/BP_PlayerPawn` (`self.PlayerPawn`)))
  (set `/Game/Blueprints/BP_PlayerPawn.CanCancel` true _asbp_player_pawn)
  (`/Game/Blueprints/BP_PlayerPawn.ResetCombo` _asbp_player_pawn)
  (`/Game/Blueprints/BP_CombatComponent.Reset` (`/Game/Blueprints/BP_PlayerPawn.CombatComponent` _asbp_player_pawn)))

(event `BeginAttack`
  (params (AttackClass :type "/Game/Blueprints/BP_Attack Class Reference") (AttackData :type "AttackData Object Reference")))