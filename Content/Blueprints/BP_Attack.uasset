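; BP_Attack is a base attack Blueprint that finds the player pawn and exposes damage, pushback and knockup values from AttackData.
; Begin, Update and End are empty hooks, with UpdateAttack running every tick.
; CheckCollisions scans Hitbox overlaps, passing itself to training dummies' TakeDamage and applying standard damage to other actors.
; ApplyMovement replaces player velocity with a mesh-relative lunge impulse when no enemy is in range.
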(event `self.ReceiveBeginPlay`
  (`/Engine/EditorBlueprintResources/StandardMacros.IsValid` (`self.PlayerPawn`)
    (:`Is Not Valid`
      (bind _asbp_player_pawn (cast `/Game/Blueprints/BP_PlayerPawn` (`GameplayStatics.GetPlayerPawn` 0)))
      (set `self.PlayerPawn` _asbp_player_pawn))))

(event `self.ReceiveTick`
  (params (DeltaSeconds :type "Float (single-precision)"))
  (`self.UpdateAttack`))

(fn `ApplyMovement`
  (params (ForwardDirection :type "Vector Structure"))
  (bind (_attackdisplacementforces_x _attackdisplacementforces_y _attackdisplacementforces_z) (`KismetMathLibrary.BreakVector` (`AttackData.AttackDisplacementForces` (`self.AttackData`))))
  (bind _skeletalmesh (`PlayerPawn.SkeletalMesh` (`self.PlayerPawn`)))
  (bind _capsulecomponent (`PlayerPawn.CapsuleComponent` (`self.PlayerPawn`)))
  (if (not (`/Game/Blueprints/BP_PlayerPawn.IsEnemyInRange` (`self.PlayerPawn`)))
    (`PrimitiveComponent.SetAllPhysicsLinearVelocity` _capsulecomponent (0.0 0.0 0.0) false)
    (`PrimitiveComponent.AddImpulse` _capsulecomponent (+ (* ForwardDirection _attackdisplacementforces_x) (* (`SceneComponent.GetRightVector` _skeletalmesh) _attackdisplacementforces_y) (* (`SceneComponent.GetUpVector` _skeletalmesh) _attackdisplacementforces_z)) "None" true)))

(fn `BeginAttack`)

(fn `CheckCollisions`
  (for _array_element (`PrimitiveComponent.GetOverlappingActors` (`self.Hitbox`) null)
    (if (!= _array_element self)
      (bind _asbp_training_dumby (cast `/Game/Blueprints/BP_TrainingDumby` _array_element)
        (:`then`
          (`self.DamageTarget` _asbp_training_dumby))
        (:`CastFailed`
          (`GameplayStatics.ApplyDamage` _array_element (`AttackData.BaseDamage` (`self.AttackData`))))))))

(fn `DamageTarget`
  (params (Target :type "/Game/Blueprints/BP_TrainingDumby Object Reference"))
  (`/Game/Blueprints/BP_TrainingDumby.TakeDamage` Target self))

(fn `EndAttack`)

(fn `GetDamageValue`
  (returns (Damage :type "Float (double-precision)"))
  (return (`AttackData.BaseDamage` (`self.AttackData`))))

(fn `GetPushbackAndKnockupForces`
  (returns (PushbackForce :type "Float (double-precision)") (KnockupForce :type "Float (double-precision)"))
  (bind _attackdata (`self.AttackData`))
  (return (`AttackData.PushbackForce` _attackdata) (`AttackData.KnockupForce` _attackdata)))

(fn `UpdateAnimSectionStatus`
  (set `self.CurrentMontageSection` "None"))

(fn `UpdateAttack`)

(fn `UserConstructionScript`)