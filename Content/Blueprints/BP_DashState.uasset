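; Player dash state that launches the pawn along its move direction and hands control back to idle when the dash ends.
; On enter, it applies a mass-independent velocity-change impulse to the capsule, scaled by DashForce, sets the locomotion state to Dash and starts a fixed timer.
; Tick counts the timer down and requests PlayerIdleState from the pawn's state machine once it runs out.
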(event `self.ReceiveTick`
  (params (DeltaSeconds :type "Float (single-precision)"))
  (bind _output_get (set `self.DashTimer` (- (`self.DashTimer`) DeltaSeconds)))
  (if (<= _output_get 0.0)
    (`StateMachine.Request` (`PlayerPawn.PlayerStateMachine` (`self.PlayerPawn`)) "/Script/PilgrimageUnreal.PlayerIdleState")))

(event `self.EnterState`
  (bind _playerpawn (`self.PlayerPawn`))
  (bind _returnvalue (`PlayerPawn.GetMoveDirection` _playerpawn))
  (`PrimitiveComponent.AddImpulse` (`PlayerPawn.CapsuleComponent` _playerpawn) (* _returnvalue (`self.DashForce`)) "None" true)
  (`PlayerPawn.SetLocomotionState` (`self.PlayerPawn`) "Dash")
  (set `self.DashTimer` 5.0))