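; Player pawn controller that records X and B button input into a frame-counted input buffer for other logic to query.
; Presses enter the buffer with a lifetime, while a per-button state map tracks held status and frame count.
; Tick ages and expires entries and increments hold counts; WasButtonPressed and IsButtonHeld expose the results.
; Joystick reading and pause-input insertion are unfinished stubs.
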(event `self.ReceiveTick`
  (params (DeltaSeconds :type "Float (single-precision)"))
  (`self.UpdateBuffer`)
  (`self.GetJoystickInput`))

(event `InputAction|X_Button`
  (params (Key :type "Key Structure"))
  (:`Pressed`
    (`self.AddInputToBuffer` "NewEnumerator0"))
  (:`Released`
    (`self.AddInputToBuffer` "NewEnumerator0" "NewEnumerator2")))

(event `InputAction|B_Button`
  (params (Key :type "Key Structure"))
  (:`Pressed`
    (`self.AddInputToBuffer` "NewEnumerator2"))
  (:`Released`
    (`self.AddInputToBuffer` "NewEnumerator2" "NewEnumerator2")))

(fn `AddInputToBuffer`
  (params (Key :type "/Game/Blueprints/E_InputBufferKey Enum" :default "NewEnumerator0") (InputType :type "/Game/Blueprints/E_InputType Enum" :default "NewEnumerator0"))
  (switch `/Game/Blueprints/E_InputType` InputType
    (:`NewEnumerator0`
      (`KismetArrayLibrary.Array_Add` (`self.InputBuffer`) (make `/Game/Blueprints/ST_InputBufferValue` Key InputType (`self.KeyPressLifetime`)))
      (`BlueprintMapLibrary.Map_Add` (`self.ButtonStates`) (`local.Key`) (make `/Game/Blueprints/ST_ButtonState` true))
      (set `self.FramesForPause` 0))
    (:`NewEnumerator2`
      (`BlueprintMapLibrary.Map_Add` (`self.ButtonStates`) (`local.Key`) (make `/Game/Blueprints/ST_ButtonState` false)))))

(fn `GetJoystickInput`
  (if (> (`self.GetInputAxisValue`) 0.3)
    _
    (elif true
      _)))

(fn `IsButtonHeld`
  (params (Button :type "/Game/Blueprints/E_InputBufferKey Enum" :default "NewEnumerator0"))
  (returns (IsHeld :type Boolean) (FramesHeld :type Integer))
  (bind (_value _returnvalue) (`BlueprintMapLibrary.Map_Find` (`self.ButtonStates`) Button))
  (if _returnvalue
    (return (break `/Game/Blueprints/ST_ButtonState` _value) (`.FramesHeld_16_A54F977A4265998173C9D2AB3E704EB1` (break `/Game/Blueprints/ST_ButtonState` _value)))
    (else
      (return false 0))))

(fn `UpdateBuffer`
  (bind _inputbuffer (`self.InputBuffer`))
  (bind _returnvalue (- (`KismetArrayLibrary.Array_Length` _inputbuffer) 1))
  (for _index (range (+ _returnvalue 1))
    (bind (_output_key _output_inputtype _output_lifetime _output_framesinbuffer) (break `/Game/Blueprints/ST_InputBufferValue` (`|GetArrayItem` _inputbuffer _index)))
    (bind _result (`/Engine/EditorBlueprintResources/StandardMacros.IncrementInt` _output_framesinbuffer)
      (:`  `
        (if (<= _output_lifetime _result)
          (`KismetArrayLibrary.Array_Remove` (`self.InputBuffer`) _index)
          (elif (and (== _index _returnvalue) (== _result (`self.FramesForPause`)))
            _)))))
  (bind _keys (`BlueprintMapLibrary.Map_Keys` (`self.ButtonStates`)))
  (for _array_element _keys
    (bind _value (`BlueprintMapLibrary.Map_Find` (`self.ButtonStates`) _array_element))
    (if (break `/Game/Blueprints/ST_ButtonState` _value)
      (`BlueprintMapLibrary.Map_Add` (`self.ButtonStates`) _array_element (make `/Game/Blueprints/ST_ButtonState` true (+ (`.FramesHeld_16_A54F977A4265998173C9D2AB3E704EB1` (break `/Game/Blueprints/ST_ButtonState` _value)) 1))))))

(fn `UserConstructionScript`)

(fn `WasButtonPressed`
  (params (ButtonKey :type "/Game/Blueprints/E_InputBufferKey Enum" :default "NewEnumerator0"))
  (returns (WasPressed :type Boolean))
  (for _array_element (`self.InputBuffer`)
    (if (`|EnumEquality` (break `/Game/Blueprints/ST_InputBufferValue` _array_element) ButtonKey)
      (return true)))
  (return false))