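; Player pawn with momentum-style movement and a double jump, including a hold-to-extend first jump.
; Tick ramps speed up with input and damps it without, feeding AddMovementInput along the last actor-relative direction, and applies jump force while held, up to a time limit.
; Each jump press flips downward physics velocity upward.
; A downward line trace resets the jump count after a short delay; debug prints and trace drawing remain active.
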(event `self.ReceiveTick`
  (params (DeltaSeconds :type "Float (single-precision)"))
  (bind (_inputvector_x _inputvector_y) (`KismetMathLibrary.BreakVector` (`self.GetMovementInput`)))
  (bind _movespeed (`self.MoveSpeed`))
  (`|ExecutionSequence`
    (:`then_0`
      (if (== (`self.GetMovementInput`) (0.0 0.0 0.0))
        (set `self.MoveSpeed` (`KismetMathLibrary.FClamp` (- (`self.MoveSpeed`) (* (`self.damping`) (`GameplayStatics.GetWorldDeltaSeconds`))) 0.0 (`self.maxSpeed`)))
        (else
          (set `self.previnput` (+ (* (`self.GetActorForwardVector`) (* _inputvector_x -1.0)) (* (`self.GetActorRightVector`) _inputvector_y)))
          (set `self.MoveSpeed` (`KismetMathLibrary.FClamp` (+ (* (+ (`self.baseSpeed`) (`self.acceleration`)) (`GameplayStatics.GetWorldDeltaSeconds`)) (`self.MoveSpeed`)) 0.0 (`self.maxSpeed`))))))
    (:`then_1`
      (`self.AddMovementInput` (`self.previnput`) _movespeed)
      (`KismetSystemLibrary.PrintString` (`KismetStringLibrary.Conv_DoubleToString` _movespeed)))
    (:`then_2`
      (if (`self.jumpHeld`)
        (`self.AddMovementInput` (`self.jumpDirection`) (`self.jumpForce`) true)
        (if (<= (`self.maxHoldTime`) (`PlayerController.GetInputKeyTimeDown` (`GameplayStatics.GetPlayerController` 0) (stale `InputAction|Jump` Key)))
          (set `self.jumpHeld` false))))
    (:`then_3`
      (bind (_hit _isgrounded) (`self.CheckIfGrounded`))
      (`KismetSystemLibrary.PrintString` (`KismetStringLibrary.Conv_BoolToString` _isgrounded) true true (struct :`R` 0.315815 :`G` 0.136861 :`B` 1.0 :`A` 1.0))
      (if (and _isgrounded (> (`self.numJumps`) 0))
        (`KismetSystemLibrary.Delay` 0.5)
        (`self.ResetJump`)))))

(event `InputAction|Jump`
  (params (Key :type "Key Structure"))
  (bind _numjumps (`self.numJumps`))
  (:`Pressed`
    (if (not (>= (`self.numJumps`) 2))
      (bind _returnvalue (`PrimitiveComponent.GetPhysicsLinearVelocity` (`self.MeshComponent`) "None"))
      (`PrimitiveComponent.SetAllPhysicsLinearVelocity` (`self.MeshComponent`) (`KismetMathLibrary.MakeVector` (.x _returnvalue) (.y _returnvalue) (* (.z _returnvalue) (`KismetMathLibrary.SignOfFloat` (.z _returnvalue)))) false)
      (`self.AddMovementInput` (`self.jumpDirection`) (`self.jumpForce`) true)
      (if (<= _numjumps 0)
        (set `self.jumpHeld` true))
      (`/Engine/EditorBlueprintResources/StandardMacros.IncrementInt` _numjumps)))
  (:`Released`
    (set `self.jumpHeld` false)))

(event `self.MeshComponent.OnComponentHit`
  (params (HitComponent :type "PrimitiveComponent Object Reference") (OtherActor :type "Actor Object Reference") (OtherComp :type "PrimitiveComponent Object Reference") (NormalImpulse :type "Vector Structure") (Hit :type "HitResult Structure (by ref)")))

(fn `CheckIfGrounded`
  (returns (Hit :type "HitResult Structure") (IsGrounded :type Boolean))
  (bind _returnvalue (`SceneComponent.K2_GetComponentLocation` (`self.MeshComponent`)))
  (bind (_outhit _returnvalue_2) (`KismetSystemLibrary.LineTraceSingleByProfile` :`Start` _returnvalue :`End` (+ _returnvalue (* (`KismetMathLibrary.NegateVector` (`self.GetActorUpVector`)) (`self.raycastDistance`))) :`ProfileName` "BlockAll" :`DrawDebugType` "Persistent"))
  (return _outhit _returnvalue_2))

(fn `ResetJump`
  (set `self.numJumps` 0))

(fn `UserConstructionScript`)