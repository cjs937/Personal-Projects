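; BP_TrainingDumby is a training dummy actor that reacts to attacks with knockback and a brief hit flash.
; TakeDamage zeroes the Collider's velocity, applies an impulse built from the attack's direction, pushback and knockup forces, then applies the attack's damage to itself.
; The resulting AnyDamage event swaps the Cylinder's material for a fraction of a second; no health is tracked.
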(event `self.ReceiveAnyDamage`
  (params (Damage :type "Float (single-precision)") (DamageType :type "DamageType Object Reference") (InstigatedBy :type "Controller Object Reference") (DamageCauser :type "Actor Object Reference"))
  (`PrimitiveComponent.SetMaterial` (`self.Cylinder`) 0 "/Engine/BasicShapes/BasicShapeMaterial.BasicShapeMaterial")
  (`KismetSystemLibrary.Delay` 0.08)
  (`PrimitiveComponent.SetMaterial` (`self.Cylinder`) 0 "/Engine/MapTemplates/Materials/BasicAsset01.BasicAsset01"))

(fn `TakeDamage`
  (params (Attack :type "/Game/Blueprints/BP_Attack Object Reference"))
  (bind (_pushbackforce _knockupforce) (`/Game/Blueprints/BP_Attack.GetPushbackAndKnockupForces` Attack))
  (bind _collider (`self.Collider`))
  (`PrimitiveComponent.SetAllPhysicsLinearVelocity` _collider (0.0 0.0 0.0) false)
  (`PrimitiveComponent.AddImpulse` _collider (+ (* (`/Game/Blueprints/BP_Attack.Direction` Attack) _pushbackforce) (* (`KismetMathLibrary.Vector_Up`) _knockupforce)) "None" true)
  (`GameplayStatics.ApplyDamage` self (`/Game/Blueprints/BP_Attack.GetDamageValue` Attack)))

(fn `UserConstructionScript`)